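; BP_Light is a fake light actor that tells the player when they enter or leave its radius.
; The construction script scales a plane to the Radius, sets the trigger sphere slightly smaller, and tints a dynamic circle fake-light material with the light color.
; Sphere begin and end overlaps call EhOnOverlapLight on BP_Player, passing itself to be added to or removed from a list.
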(event `self.ReceiveBeginPlay`)

(event `self.Sphere.OnComponentBeginOverlap`
  (params (OverlappedComponent :type "PrimitiveComponent Object Reference") (OtherActor :type "Actor Object Reference") (OtherComp :type "PrimitiveComponent Object Reference") (OtherBodyIndex :type Integer) (bFromSweep :type Boolean) (SweepResult :type "HitResult Structure (by ref)"))
  (bind _asbp_player (cast `/Game/_UE4Spring19/Core/Game/BP_Player` OtherActor))
  (`/Game/_UE4Spring19/Core/Game/BP_Player.eh_OnOverlapLight` _asbp_player true self))

(event `self.Sphere.OnComponentEndOverlap`
  (params (OverlappedComponent :type "PrimitiveComponent Object Reference") (OtherActor :type "Actor Object Reference") (OtherComp :type "PrimitiveComponent Object Reference") (OtherBodyIndex :type Integer))
  (bind _asbp_player (cast `/Game/_UE4Spring19/Core/Game/BP_Player` OtherActor))
  (`/Game/_UE4Spring19/Core/Game/BP_Player.eh_OnOverlapLight` _asbp_player false self))

(fn `UserConstructionScript`
  (bind _radius (`self.Radius`))
  (bind _returnvalue (/ _radius 50.0))
  (`SphereComponent.SetSphereRadius` (`self.Sphere`) (* _radius 0.7) true)
  (`SceneComponent.SetWorldScale3D` (`self.Plane`) (`KismetMathLibrary.MakeVector` _returnvalue _returnvalue _returnvalue))
  (bind _returnvalue_2 (`PrimitiveComponent.CreateDynamicMaterialInstance` (`self.Plane`) 0 "/Game/_UE4Spring19/Art/MI_FakeLight_Circle.MI_FakeLight_Circle" "None"))
  (bind _output_get (set `self.FakeLight_DMI` _returnvalue_2))
  (`MaterialInstanceDynamic.SetVectorParameterValue` _output_get "LightColor" (`self.Lightcolor`)))
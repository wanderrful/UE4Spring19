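; BP_Game_C is an enemy character that fires a weapon at the player.
; On BeginPlay it spawns a FIDEO_Weapon and snaps it to the GunTemp component.
; eh_OnAttackPlayer stops movement, snaps yaw toward the given player, prints a debug "PEW!", sets Enemyspotted1 and calls Fire on the weapon.
; ABP_Deer casts and trigger pull/release nodes are disconnected leftovers that never run.
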(event `eh_OnAttackPlayer`
  (params (PlayerRef :type "/Game/_UE4Spring19/Core/Game/BP_Player Object Reference"))
  (bind (_returnvalue_roll _returnvalue_pitch _returnvalue_yaw) (`KismetMathLibrary.BreakRotator` (`KismetMathLibrary.FindLookAtRotation` (`self.K2_GetActorLocation`) (`self.K2_GetActorLocation` PlayerRef))))
  (`NavMovementComponent.StopActiveMovement` (`self.CharacterMovement`))
  (`self.K2_SetActorRotation` (`KismetMathLibrary.MakeRotator` 0.0 0.0 _returnvalue_yaw)) ; TODO: Lerp this, instead of snapping!
  (`KismetSystemLibrary.PrintString` "PEW!" true true (struct :`R` 1.0 :`G` 0.109179 :`A` 1.0))
  (set `self.Enemyspotted1` true)
  (`/Game/_UE4Spring19/Core/Game/AI/FIDEO_Weapon.Fire` (`self.Weapon`)))

(event `self.ReceiveBeginPlay`
  (bind _guntemp (`self.GunTemp`))
  ;[1 1 1] Fideo's Projectile
  (`|ExecutionSequence`
    (:`then_0`
      (bind _returnvalue (`|SpawnActorFromClass` "/Game/_UE4Spring19/Core/Game/AI/FIDEO_Weapon.FIDEO_Weapon_C" (`SceneComponent.K2_GetComponentToWorld` _guntemp) "Undefined" "OverrideRootScale" null null))
      (bind _output_get (set `self.Weapon` _returnvalue))
      (`self.K2_AttachToComponent` _output_get _guntemp "None" "SnapToTarget" "SnapToTarget" "KeepWorld" true))))

(fn `UserConstructionScript`)
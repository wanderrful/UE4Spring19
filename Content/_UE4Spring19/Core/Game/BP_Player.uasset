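; BP_Player is the player Blueprint for a stealth game, tracking light-based visibility and health.
; Lights are added or removed through an overlap handler, and a looping timer set on BeginPlay drives periodic visibility checks.
; Visibility follows the light with the smallest horizontal distance relative to its scaled radius, rising toward its center.
; It also creates the stealth meter widget and signals player death when damage depletes health.
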(event `self.ReceiveBeginPlay`
  (`parent.ReceiveBeginPlay`)
  (`KismetSystemLibrary.Delay` 0.2)
  (`|ExecutionSequence`
    (:`then_0`
      (bind _returnvalue (`KismetSystemLibrary.K2_SetTimerDelegate` (`|CreateDelegate` :!event `eh_OnLightCheckTimer`) 0.1 true))
      (set `self.LightCheckTimer` _returnvalue))
    (:`then_1`
      (bind _asbp_game_pc (cast `/Game/_UE4Spring19/Core/Game/BP_Game_PC` (`self.GetController`)))
      (bind _returnvalue_2 (`|CreateWidget` "/Game/_UE4Spring19/UI/WB_StealthMeter.WB_StealthMeter_C" _asbp_game_pc))
      (`UserWidget.AddToViewport` _returnvalue_2 0))))

(event `eh_OnOverlapLight`
  (params (bAddToList :type Boolean) (Light :type "/Game/_UE4Spring19/Core/Game/BP_Light Object Reference"))
  (bind _lights (`self.Lights`))
  (if bAddToList
    (`KismetArrayLibrary.Array_AddUnique` _lights Light)
    (else
      (`KismetArrayLibrary.Array_RemoveItem` _lights Light))))

(event `eh_OnLightCheckTimer`
  (`|ExecutionSequence`
    (:`then_0`
      (bind _returnvalue (`self.fn_CalculateVisibilityLevel` (`self.Lights`)))
      (set `self.VisibilityLevel` _returnvalue))))

(event `OnReceiveDamage`
  (params (DamageAmount :type "Float (double-precision)"))
  (bind _output_get (set `self.Health` (- (`self.Health`) DamageAmount)))
  (if (<= _output_get 0.0)
    (`self.OnPlayerDeath`)))

(fn `fn_CalculateVisibilityLevel`
  (params (Lights :type "Array of /Game/_UE4Spring19/Core/Game/BP_Light Object Reference"))
  (returns (ReturnValue :type "Float (double-precision)"))
  (locals (Percentages :type "Array of Float (double-precision)"))
  (if (< (`KismetArrayLibrary.Array_Length` Lights) 1)
    (return 0.0)
    (else
      (for _array_element Lights
        (`KismetArrayLibrary.Array_Add` (`local.Percentages`) (`KismetMathLibrary.FClamp` (/ (`self.GetHorizontalDistanceTo` _array_element self) (* (`/Game/_UE4Spring19/Core/Game/BP_Light.Radius` _array_element) 0.7)))))
      (return (- 1.0 (`.MinValue` (`KismetMathLibrary.MinOfFloatArray` (`local.Percentages`))))))))

(fn `UserConstructionScript`
  (`parent.UserConstructionScript`))
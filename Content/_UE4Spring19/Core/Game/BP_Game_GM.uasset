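; BP_Game_GM is the game mode that tracks which AI can see the player and relays music and victory events.
; Spotted events add or remove AI controller references in a unique list.
; When a music reset is tried, it tells the player controller to switch to normal music only if that list is empty.
; Victory is passed straight through to the game instance.
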(event `eh_OnTryMusicReset`
  (if (<= (`KismetArrayLibrary.Array_Length` (`self.GuysWhoSeePlayer`)) 0)
    (bind _asbp_game_pc (cast `/Game/_UE4Spring19/Core/Game/BP_Game_PC` (`GameplayStatics.GetPlayerController` 0)))
    (`/Game/_UE4Spring19/Core/Game/BP_Game_PC.eh_OnSwitchToNormalMusic` _asbp_game_pc)))

(event `eh_OnPlayerSpotted`
  (params (AICRef :type "AIController Object Reference") (CanSeePlayer :type Boolean))
  (bind _guyswhoseeplayer (`self.GuysWhoSeePlayer`))
  (if CanSeePlayer
    (`KismetArrayLibrary.Array_AddUnique` _guyswhoseeplayer AICRef)
    (else
      (`KismetArrayLibrary.Array_RemoveItem` _guyswhoseeplayer AICRef))))

(event `eh_OnVictory`
  (bind _asbp_game_gi (cast `/Game/_UE4Spring19/Core/BP_Game_GI` (`GameplayStatics.GetGameInstance`)))
  (`/Game/_UE4Spring19/Core/BP_Game_GI.eh_OnVictory` _asbp_game_gi))

(fn `UserConstructionScript`)
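; Player controller for a game jam project that toggles the pause menu widget from the PauseGame input.
; On BeginPlay it focuses the game viewport; the pause event creates the widget on first use, then reuses it.
; Showing the menu switches to UI-only input focused on it and hides the cursor, while removing it restores game-only input and shows the cursor.
; It only handles menu and input mode, without pausing the game itself.
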(event `self.ReceiveBeginPlay`
  (`WidgetBlueprintLibrary.SetFocusToGameViewport`))

(event `eh_OnPauseGame`
  (bind _ui_pause (`self.UI_Pause`)
    (:`then`
      (if (`Widget.IsInViewport` _ui_pause)
        (`Widget.RemoveFromParent` _ui_pause)
        (`WidgetBlueprintLibrary.SetInputMode_GameOnly` self)
        (set `self.bShowMouseCursor` true)
        (else
          (`UserWidget.AddToViewport` _ui_pause 1)
          (`WidgetBlueprintLibrary.SetInputMode_UIOnlyEx` self (`self.UI_Pause`) :!label _label)
          (set `self.bShowMouseCursor` false))))
    (:`else`
      (bind _returnvalue (`|CreateWidget` "/Game/GameJamKit/Blueprints/UMG/UMG_GameJam_PauseMenu_Widget.UMG_GameJam_PauseMenu_Widget_C" self))
      (bind _output_get (set `self.UI_Pause` _returnvalue))
      (`UserWidget.AddToViewport` _output_get 1)
      (goto _label))))

(event `InputAction|PauseGame`
  (params (Key :type "Key Structure"))
  (:`Pressed`
    (`self.eh_OnPauseGame`)))

(fn `UserConstructionScript`)
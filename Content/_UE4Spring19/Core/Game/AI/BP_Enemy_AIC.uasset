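; AI controller for enemies that runs the BT_Enemy behavior tree and feeds its blackboard for patrolling and player detection.
; Waypoint events cycle through the controlled pawn's waypoint list with wraparound, writing each location to CurrentDestination.
; A looping timer polls sight perception, setting PlayerRef only when the seen player's VisibilityLevel exceeds a threshold, otherwise clearing it.
; A helper function reports whether PlayerRef is valid.
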(event Custom|eh_onTimerCheck
  (bind _returnvalue (Utilities|Name|MakeLiteralName "PlayerRef"))
  (bind _blackboard (Variables|Default|GetBlackboard))
  (for _array_element (Class|AIPerceptionComponent|GetCurrentlyPerceivedActors (Variables|Default|GetAIPerception) "/Script/AIModule.AISense_Sight")
    (bind _asbp_player (Utilities|Casting|CastToBP_Player _array_element))
    (if (> (Variables|/Game/_UE4Spring19/Core/Game/BP_Player.BP_Player_C|GetVisibilityLevel _asbp_player) (Variables|Default|GetMinimumVisibilityToSeePlayer)) ; Even though we "see" the player...do we "really" see them?
      (AI|Components|Blackboard|SetValueasObject _blackboard _returnvalue _asbp_player)
      (else
        (AI|Components|Blackboard|ClearValue _blackboard _returnvalue)))))

(event Custom|eh_OnNextWaypoint
  (bind _asbp_game_c (Utilities|Casting|CastToBP_Game_C (Pawn|GetControlledPawn)))
  (if (> (Utilities|Array|Length (Variables|/Game/_UE4Spring19/Core/Game/BP_Game_C.BP_Game_C_C|GetWaypoints _asbp_game_c)) 0)
    (bind _output_get (Variables|Default|SetCurrentWaypointIndex (|((X+1)%Y) (Variables|Default|GetCurrentWaypointIndex) (Utilities|Array|Length (Variables|/Game/_UE4Spring19/Core/Game/BP_Game_C.BP_Game_C_C|GetWaypoints _asbp_game_c)))))
    (AI|Components|Blackboard|SetValueasVector (Variables|Default|GetBlackboard) (Utilities|Name|MakeLiteralName "CurrentDestination") (Transformation|GetActorLocation (Utilities|Array|Get(acopy) (Variables|/Game/_UE4Spring19/Core/Game/BP_Game_C.BP_Game_C_C|GetWaypoints _asbp_game_c) _output_get)))))

(event EventBeginPlay
  (Utilities|FlowControl|Sequence
    (:then_0
      (Utilities|Time|SetTimerbyEvent (EventDispatchers|CreateEvent :!event Custom|eh_onTimerCheck) 0.5 true))
    (:then_1
      (AI|RunBehaviorTree self "/Game/_UE4Spring19/Core/Game/AI/BT_Enemy.BT_Enemy"))
    (:then_2
      (bind _asbp_game_c (Utilities|Casting|CastToBP_Game_C (Pawn|GetControlledPawn)))
      (if (> (Utilities|Array|Length (Variables|/Game/_UE4Spring19/Core/Game/BP_Game_C.BP_Game_C_C|GetWaypoints _asbp_game_c)) 0)
        (CallFunction|EhonNextWaypoint)))))

(fn ConstructionScript)

(fn FnBCanSeePlayer
  (return (Utilities|IsValid (AI|Components|Blackboard|GetValueasObject (Variables|Default|GetBlackboard) (Utilities|Name|MakeLiteralName "PlayerRef")))))